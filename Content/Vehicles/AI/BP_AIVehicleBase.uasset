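; Base AI vehicle that drives at full throttle from BeginPlay and steers along a spline path or toward the player's current vehicle.
; Each tick, FollowPlayer selects the target, and the yaw difference to it is mapped to steering input.
; Path following uses a look-ahead point, projecting ahead along the spline tangent and snapping back onto the spline.
; Tick also updates the reverse-gear flag and feeds absolute forward speed into the engine's RPM parameter.
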(event `self.ReceiveBeginPlay`
  ;[1 0.04688 0.04688] Vehicle AI
  (`WheeledVehicleMovementComponent.SetThrottleInput` (`self.VehicleMovement`) 1.0))

(event `self.ReceiveTick`
  (params (DeltaSeconds :type "Float (single-precision)"))
  (bind _vehiclemovement (`self.VehicleMovement`))
  ;[1 0.04688 0.04688] Vehicle AI
  (`WheeledVehicleMovementComponent.SetSteeringInput` (`self.VehicleMovement`) (select `bool` (`self.bFollowPlayer`) :`false` (`self.Get Path`) :`true` (`self.Get Path To Player`)))
  (set `self.bInReverseGear` (< (`WheeledVehicleMovementComponent.GetCurrentGear` _vehiclemovement) 0))
  (`AudioComponent.SetFloatParameter` (`self.Engine`) "RPM" (`KismetMathLibrary.Abs` (`WheeledVehicleMovementComponent.GetForwardSpeed` _vehiclemovement))))

(fn `Get Path`
  (returns (ReturnValue :type "Float (double-precision)"))
  (bind _returnvalue (`self.K2_GetActorLocation`))
  (bind _current_path (`self.Current Path`))
  (bind _spline (`/Game/Vehicles/AI/BP_AIVehiclePath.Spline` _current_path))
  (bind (_returnvalue_roll _returnvalue_pitch _returnvalue_yaw) (`KismetMathLibrary.BreakRotator` (`KismetMathLibrary.NormalizedDeltaRotator` (`KismetMathLibrary.FindLookAtRotation` _returnvalue (`SplineComponent.FindLocationClosestToWorldLocation` _spline (+ (* (`KismetMathLibrary.Normal` (`SplineComponent.FindTangentClosestToWorldLocation` _spline _returnvalue "World")) 200.0) _returnvalue) "World")) (`self.K2_GetActorRotation`))))
  (`/Engine/EditorBlueprintResources/StandardMacros.IsValid` _current_path
    (:`Is Valid`
      (return (`KismetMathLibrary.MapRangeClamped` _returnvalue_yaw -90.0 90.0 -1.0 1.0)))))

(fn `Get Path To Player`
  (returns (ReturnValue :type "Float (double-precision)"))
  (bind (_returnvalue _vehicle_location) (`self.Get Current Vehicle`))
  (bind (_returnvalue_roll _returnvalue_pitch _returnvalue_yaw) (`KismetMathLibrary.BreakRotator` (`KismetMathLibrary.NormalizedDeltaRotator` (`KismetMathLibrary.FindLookAtRotation` (`self.K2_GetActorLocation`) _vehicle_location) (`self.K2_GetActorRotation`))))
  (`/Engine/EditorBlueprintResources/StandardMacros.IsValid` _returnvalue
    (:`Is Valid`
      (return (`KismetMathLibrary.MapRangeClamped` _returnvalue_yaw -90.0 90.0 -1.0 1.0)))))

(fn `UserConstructionScript`)