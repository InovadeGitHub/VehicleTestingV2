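; BP_Forcefield is a world barrier that knocks vehicles away when they hit it.
; A looping timer is set on BeginPlay, and UpdateRotation turns ForceDirection using CalculateRotation while the current vehicle is valid.
; Hits apply a velocity-change impulse along that direction, with particles, sound and camera shake.
; A timeline expands an impact radius at the hit point on the dynamic material.
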(event `self.ReceiveBeginPlay`
  (bind _returnvalue (`PrimitiveComponent.CreateDynamicMaterialInstance` (`self.Forcefield`) 0 null "None"))
  (set `self.Forcefield Material` _returnvalue)
  (`KismetSystemLibrary.K2_SetTimerDelegate` (`|CreateDelegate` :!event `Update Rotation`) 0.01 true))

(event `Update Rotation`
  (`/Engine/EditorBlueprintResources/StandardMacros.IsValid` (`/Game/Blueprints/Core/BP_FunctionLibrary.Get Current Vehicle`)
    (:`Is Valid`
      (`SceneComponent.K2_SetWorldRotation` (`self.Force Direction`) (`self.Calculate Rotation`) false false))))

(event `self.Forcefield.OnComponentHit`
  (params (HitComponent :type "PrimitiveComponent Object Reference") (OtherActor :type "Actor Object Reference") (OtherComp :type "PrimitiveComponent Object Reference") (NormalImpulse :type "Vector Structure") (Hit :type "HitResult Structure (by ref)"))
  (bind _forcefield_material (`self.Forcefield Material`))
  ;[1 0.09896 0.09896] Forcefield Logic
  (bind _asbp_base_vehicle (cast `/Game/Vehicles/Player/BP_BaseVehicle` OtherActor))
  (`PrimitiveComponent.AddImpulse` (`WheeledVehicle.Mesh` _asbp_base_vehicle) (* (`SceneComponent.GetForwardVector` (`self.Force Direction`)) (`self.Push Force`)) "None" true)
  (`MaterialInstanceDynamic.SetVectorParameterValue` _forcefield_material "Impact Location" (`KismetMathLibrary.Conv_VectorToLinearColor` Hit_Location))
  (bind _returnvalue (`GameplayStatics.SpawnEmitterAtLocation` "/Game/Effects/ForcefieldImpact/P_ForcefieldImpact.P_ForcefieldImpact" Hit_Location))
  (`|ExecutionSequence`
    (:`then_0`
      (`GameplayStatics.PlaySoundAtLocation` null Hit_Location (struct) 1.0 1.0 0.0 null null null)
      (`PlayerCameraManager.StartCameraShake` :`self` (`GameplayStatics.GetPlayerCameraManager` 0) :`PlaySpace` "World")
      (bind (_direction _impact_radius) (`Timeline|TL_ForcefieldHit` :!via `PlayFromStart`)
        (:`Update`
          (`MaterialInstanceDynamic.SetScalarParameterValue` _forcefield_material "Impact Radius" (`KismetMathLibrary.Lerp` 0.0 100.0 _impact_radius)))))
    (:`then_1`
      (`KismetSystemLibrary.Delay` 1.0)
      (`ActorComponent.K2_DestroyComponent` _returnvalue))))

(fn `UserConstructionScript`
  (if (`self.bDebug`)
    (`SceneComponent.SetHiddenInGame` (`self.Force Direction`) false false)))