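; Actor component for physics items that plays an impact sound on collision and toggles the item's held state.
; It binds to the owner's static mesh hit event and ignores impacts briefly after BeginPlay.
; A DoOnce with a randomized delayed reset throttles the sound, which requires a minimum mesh speed.
; ToggleHolding switches physics simulation, collision and Pawn blocking off while held and back on when released.
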(event `self.ReceiveBeginPlay`
  (bind _returnvalue (`Actor.GetComponentByClass` (`self.GetOwner`) "/Script/Engine.StaticMeshComponent"))
  (`/Engine/EditorBlueprintResources/StandardMacros.IsValid` _returnvalue
    (:`Is Valid`
      (set `self.MeshComponent` _returnvalue)
      (add `PrimitiveComponent.OnComponentHit` (`self.MeshComponent`) (`|CreateDelegate` :!event `On Hit`)))
    (:`Is Not Valid`
      _))
  (`KismetSystemLibrary.Delay` 0.5)
  (set `self.bCanImpact` true))

(event `On Hit`
  (params (HitComponent :type "PrimitiveComponent Object Reference") (OtherActor :type "Actor Object Reference") (OtherComp :type "PrimitiveComponent Object Reference") (NormalImpulse :type "Vector Structure") (Hit :type "HitResult Structure (by ref)"))
  (if (`self.bCanImpact`)
    (`|ExecutionSequence`
      (:`then_0`
        (`KismetSystemLibrary.Delay` (`KismetMathLibrary.RandomFloatInRange` 0.4 0.7))
        (goto _label :!via `Reset`))
      (:`then_1`
        (`/Engine/EditorBlueprintResources/StandardMacros.DoOnce` false :!label _label
          (:`Completed`
            (if (>= (`self.Get Item Speed`) 60.0)
              (`GameplayStatics.SpawnSoundAtLocation` (`self.Impact Sound`) (`SceneComponent.K2_GetComponentLocation` (`self.MeshComponent`)) (struct) 1.0 1.0 0.0 null null))))))))

(fn `Get Item Speed`
  (returns (ReturnValue :type "Float (double-precision)"))
  (return (`KismetMathLibrary.VSize` (`SceneComponent.GetComponentVelocity` (`self.MeshComponent`)))))

(fn `Toggle Holding`
  (params (Holding :type Boolean))
  (bind _meshcomponent (`self.MeshComponent`))
  (`PrimitiveComponent.SetSimulatePhysics` _meshcomponent (not Holding))
  (`PrimitiveComponent.SetCollisionResponseToChannel` _meshcomponent "ECC_Pawn" (select `bool` Holding :`false` "ECR_Block" :`true` "ECR_Ignore" :!type "ECollisionResponse Enum"))
  (`PrimitiveComponent.SetCollisionEnabled` (`self.MeshComponent`) (select `bool` Holding :`false` "QueryAndPhysics" :`true` "NoCollision" :!type "ECollisionEnabled Enum")))