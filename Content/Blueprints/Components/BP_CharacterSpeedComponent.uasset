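; Actor component that sets the owning Character's walking and crouching movement speeds.
; On BeginPlay it caches the CharacterMovement component and applies its default Walk and Crouch speeds through UpdateSpeed.
; UpdateSpeed skips any zero input, otherwise clamps the value between the min and max speeds, scales it by Factor and writes it to MaxWalkSpeed or MaxWalkSpeedCrouched.
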(event `self.ReceiveBeginPlay`
  (set `self.Character Movement` (`Character.CharacterMovement` (cast `Character` (`self.GetOwner`) :!pure true)))
  (`self.Update Speed` (`self.Walk`) (`self.Crouch`)))

(fn `Update Speed`
  (params (`Walking Speed` :type "Float (double-precision)") (`Crouching Speed` :type "Float (double-precision)"))
  (if (not (== `Walking Speed` 0.0))
    (set `CharacterMovementComponent.MaxWalkSpeed` (* (`KismetMathLibrary.FClamp` (`local.Walking Speed`) (`self.MinSpeed`) (`self.MaxSpeed`)) (`self.Factor`)) (`self.Character Movement`)))
  (if (not (== `Crouching Speed` 0.0))
    (set `CharacterMovementComponent.MaxWalkSpeedCrouched` (* (`KismetMathLibrary.FClamp` (`local.Crouching Speed`) (`self.MinSpeed`) (`self.MaxSpeed`)) (`self.Factor`)) (`self.Character Movement`))))