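; Blueprint function library of shared helpers for vehicle lookup, proximity search and random vectors.
; GetCurrentVehicle casts player pawn 0 to BP_BaseVehicle, stopping if the cast fails, with a first-vehicle-in-world fallback if the result is invalid.
; GetNearestActorOfClass linearly scans all actors of a class for the one closest to a location, returning it and its distance.
; RandomVectorInRange randomizes each axis independently between shared bounds.
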(fn `Get Current Vehicle`
  (returns (ReturnValue :type "/Game/Vehicles/Player/BP_BaseVehicle Object Reference"))
  (bind _asbp_base_vehicle (cast `/Game/Vehicles/Player/BP_BaseVehicle` (`GameplayStatics.GetPlayerPawn` null)))
  (`/Engine/EditorBlueprintResources/StandardMacros.IsValid` _asbp_base_vehicle
    (:`Is Valid`
      (return _asbp_base_vehicle))
    (:`Is Not Valid`
      (bind _outactors (`GameplayStatics.GetAllActorsOfClass` null "/Game/Vehicles/Player/BP_BaseVehicle.BP_BaseVehicle_C"))
      (return (`|GetArrayItem` _outactors)))))

(fn `Get Nearest Actor Of Class`
  (params (`Actor Class` :type "Actor Class Reference") (`Search Location` :type "Vector Structure"))
  (returns (`Nearest Actor` :type "Actor Object Reference") (`Nearest Distance` :type "Float (double-precision)"))
  (locals (`Nearest Distance From Search Location` :type "Float (double-precision)" :default 10000.0) (`Nearest Actor Of Class` :type "Actor Object Reference"))
  (bind _outactors (`GameplayStatics.GetAllActorsOfClass` null `Actor Class`))
  (for _array_element _outactors
    (bind _returnvalue (`KismetMathLibrary.Vector_Distance` (`Actor.K2_GetActorLocation` _array_element) (`local.Search Location`)))
    (if (< _returnvalue (`local.Nearest Distance From Search Location`))
      (set `local.Nearest Distance From Search Location` _returnvalue)
      (set `local.Nearest Actor Of Class` _array_element)))
  (return (`local.Nearest Actor Of Class`) (`local.Nearest Distance From Search Location`)))

(fn `Random Vector In Range`
  (params (Min :type "Float (double-precision)") (Max :type "Float (double-precision)" :default 0.0))
  (returns (ReturnValue :type "Vector Structure"))
  (bind _returnvalue (`KismetMathLibrary.RandomFloatInRange` Min Max))
  (return (`KismetMathLibrary.MakeVector` _returnvalue _returnvalue _returnvalue)))